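; BP_Blocks is a grid of breakable blocks that BP_Ball hits, apparently for a Breakout-style game.
; The construction script lays out static mesh components in an X-by-Y grid spaced by Padding.
; Each block's material doubles as its health: the first ball hit turns it to rusted metal, the next destroys that component.
; Destroyed blocks randomly spawn a BP_Bonus at their transform, weighted by BonusChance.
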(event EventBeginPlay)

(event Collision|EventActorBeginOverlap
  (params (OtherActor :type Actor%20Object%20Reference)))

(event Collision|EventHit
  (params (MyComp :type Primitive%20Component%20Object%20Reference) (Other :type Actor%20Object%20Reference) (OtherComp :type Primitive%20Component%20Object%20Reference) (bSelfMoved :type Boolean) (HitLocation :type Vector :default "0, 0, 0") (HitNormal :type Vector :default "0, 0, 0") (NormalImpulse :type Vector :default "0, 0, 0") (Hit :type Hit%20Result%20Structure%20%28by%20ref%29))
  (Variables|Default|SetCube MyComp)
  (Utilities|Casting|CastToBP_Ball Other)
  (CallFunction|CubeHealthPoints))

(fn ConstructionScript
  (for _index (range 0 (Variables|Default|Getx))
    (for _index_2 (range 0 (Variables|Default|Gety))
      (AddComponent|AddStaticMeshComponent false (Math|Transform|MakeTransform (Math|Vector|MakeVector (Math|Conversions|ToFloat(Integer) (* _index (Variables|Default|GetPadding))) (Math|Conversions|ToFloat(Integer) (* _index_2 (Variables|Default|GetPadding))) 0.0))))))

(fn CubeHealthPoints
  (bind _cube (Variables|Default|GetCube))
  (Development|PrintString (Utilities|GetDisplayName _cube))
  (if (== (Rendering|Material|GetMaterial _cube 0) "/Game/StarterContent/Materials/M_Metal_Rust.M_Metal_Rust")
    (Utilities|FlowControl|Sequence
      (:then_0
        (if (Math|Random|RandomBoolwithWeight (Variables|Default|GetBonusChance))
          (CallFunction|SpawnBonus)))
      (:then_1
        (Components|DestroyComponent (Variables|Default|GetCube))))
    (else
      (Rendering|Material|SetMaterial (Variables|Default|GetCube) 0 "/Game/StarterContent/Materials/M_Metal_Rust.M_Metal_Rust"))))

(fn SpawnBonus
  (bind _returnvalue (Game|SpawnActorfromClass "/Game/Main/Blueprints/BP_Bonus.BP_Bonus_C" (Transformation|GetWorldTransform (Variables|Default|GetCube)) "Undefined" 0 0))
  (Variables|Default|SetBonus _returnvalue))