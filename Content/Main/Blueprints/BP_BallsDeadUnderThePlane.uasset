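; BP_BallsDeadUnderThePlane is a functional test checking that the playing ball dies below the player's paddle cube along the X axis.
; PrepareTest caches the BP_Pawn's cube location and binds to its PlayingBall's OnDead event.
; On death, the test succeeds if the ball's sphere X is less than the cached X, and fails otherwise.
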(event Custom|OnDeadReaction
  (if (< (.x (Transformation|GetWorldLocation (Variables|/Game/Main/BP_Ball.BP_Ball_C|GetSphere (Variables|Default|GetBall)))) (.x (Variables|Default|GetPawnLoaction)))
    (Class|FunctionalTest|FinishTest "Succeeded")
    (else
      (Class|FunctionalTest|FinishTest "Failed"))))

(event EventPrepareTest
  (bind _asbp_pawn (Utilities|Casting|CastToBP_Pawn (Game|Player|GetPlayerPawn 0)))
  (Variables|Default|SetPawnLoaction (Transformation|GetWorldLocation (Variables|/Game/Main/Blueprints/BP_Pawn.BP_Pawn_C|GetCube _asbp_pawn)))
  (bind _output_get (Variables|Default|SetBall (Variables|/Game/Main/Blueprints/BP_Pawn.BP_Pawn_C|GetPlayingBall _asbp_pawn)))
  (EventDispatchers|AssignOnDead _output_get (delegate Custom|OnDeadReaction)))

(event EventStartTest)

(event EventTick
  (params (DeltaSeconds :type Float%20%28single-precision%29)))

(fn ConstructionScript)