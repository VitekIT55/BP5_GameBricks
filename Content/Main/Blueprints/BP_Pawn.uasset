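; Player pawn that slides sideways and keeps a BP_Ball in play, much like a paddle.
; On BeginPlay it spawns a ball at its capsule's transform and binds to the ball's OnDead event, which loops back to spawn and bind a replacement.
; MoveRight axis input moves the pawn along Y with swept, fixed-size offsets per update, independent of axis magnitude and frame time.
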(event Custom|OnDeadReaction
  (bind _returnvalue (Game|SpawnActorfromClass "/Game/Main/BP_Ball.BP_Ball_C" (Transformation|GetWorldTransform (Variables|Default|GetCapsule)) "AlwaysSpawn" 0 0))
  (bind _output_get (Variables|Default|SetPlayingBall _returnvalue))
  (EventDispatchers|AssignOnDead _output_get (delegate Custom|OnDeadReaction)))

(event EventBeginPlay
  (bind _returnvalue (Game|SpawnActorfromClass "/Game/Main/BP_Ball.BP_Ball_C" (Transformation|GetWorldTransform (Variables|Default|GetCapsule)) "AlwaysSpawn" 0 0))
  (bind _output_get (Variables|Default|SetPlayingBall _returnvalue))
  (EventDispatchers|AssignOnDead _output_get (delegate Custom|OnDeadReaction)))

(event Input|AxisEvents|InputAxisMoveRight
  (params (AxisValue :type Float%20%28single-precision%29))
  (if (< AxisValue 0.0)
    (Transformation|AddActorWorldOffset "0,-20.000000, 0" true)))

(event Input|AxisEvents|InputAxisMoveRight
  (params (AxisValue :type Float%20%28single-precision%29))
  (if (> AxisValue 0.0)
    (Transformation|AddActorWorldOffset "0,20.000000, 0" true)))

(fn ConstructionScript)